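; BP_Generator is a power generator with a button that the player activates by standing in its trigger.
; Trigger overlap events filter for the PlayerCharacter's capsule component and set the pressed state.
; Entering calls EnergyGain, which is not defined in these graphs, and both entering and leaving run ChangeButtonColor to swap the button between on and off materials.
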(event `self.trigger.OnComponentBeginOverlap`
  (params (OverlappedComponent :type "PrimitiveComponent Object Reference") (OtherActor :type "Actor Object Reference") (OtherComp :type "PrimitiveComponent Object Reference") (OtherBodyIndex :type Integer) (bFromSweep :type Boolean) (SweepResult :type "HitResult Structure (by ref)"))
  ;[1 1 1] The button changes collor and gains Power if is being pressed or not
  (if (and (`KismetMathLibrary.ClassIsChildOf` (`GameplayStatics.GetObjectClass` OtherActor) "/Script/SleepersHaunting.PlayerCharacter") (`GameplayStatics.ObjectIsA` OtherComp "/Script/Engine.CapsuleComponent"))
    (set `self.isPressed` true)
    (`self.EnergyGain`)
    (`self.ChangeButtonColor` :!label _label)))

(event `self.trigger.OnComponentEndOverlap`
  (params (OverlappedComponent :type "PrimitiveComponent Object Reference") (OtherActor :type "Actor Object Reference") (OtherComp :type "PrimitiveComponent Object Reference") (OtherBodyIndex :type Integer))
  ;[1 1 1] The button changes collor and gains Power if is being pressed or not
  (if (and (`KismetMathLibrary.ClassIsChildOf` (`GameplayStatics.GetObjectClass` OtherActor) "/Script/SleepersHaunting.PlayerCharacter") (`GameplayStatics.ObjectIsA` OtherComp "/Script/Engine.CapsuleComponent"))
    (set `self.isPressed` false)
    (goto _label)))

(event `ChangeButtonColor`
  (bind _button (`self.button`))
  (if (`self.isPressed`)
    (`PrimitiveComponent.SetMaterial` _button 0 "/Game/Objects/Power/Generator/m_ButtonOn.m_ButtonOn")
    (else
      (`PrimitiveComponent.SetMaterial` _button 0 "/Game/Objects/Power/Generator/m_ButtonOff.m_ButtonOff"))))

(fn `UserConstructionScript`)