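; BP_SlideDoors is a grabbable sliding door that is pushed along negative world X whenever it is not held.
; Grab and Release call their parent implementations, then set or clear the IsBeingGrabbed flag.
; Tick checks that flag and, when it is false, applies a constant physics force to SlideDoorMeshComponent, with no delta-time scaling or position check in this graph.
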(event `self.ReceiveTick`
  (params (DeltaSeconds :type "Float (single-precision)"))
  (if (`self.bIsBeingGrabbed`)
    (set `self.bIsBeingGrabbed` true)
    (else
      (`PrimitiveComponent.AddForce` (`self.SlideDoorMeshComponent`) (-10000.0 0.0 0.0) "None" false)
      (set `self.bIsBeingGrabbed` false))))

(event `GrabbableInterface.Grab`
  (`parent.Grab`)
  (set `self.bIsBeingGrabbed` true))

(event `GrabbableInterface.Release`
  (`parent.Release`)
  (set `self.bIsBeingGrabbed` false))

(fn `UserConstructionScript`)