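; Player character with a physics-driven body that can grab nearby physics objects.
; On BeginPlay, physical animation drives the bodies from the pelvis down the hierarchy, with those below the pelvis simulating physics.
; While IA_Grab triggers, a debug-drawn sphere trace at the actor's location finds a PhysicsBody and constrains it to the upper spine bone.
; Completing the input breaks the constraint and clears IsGrabbing.
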(event `self.ReceiveBeginPlay`
  (bind _pelvisbone (`self.pelvisBone`))
  (`PhysicalAnimationComponent.SetSkeletalMeshComponent` (`self.PhysicalAnimation`) (`self.Mesh`))
  (`PhysicalAnimationComponent.ApplyPhysicalAnimationSettingsBelow` (`self.PhysicalAnimation`) _pelvisbone (make `PhysicalAnimationData` true 1000.0 100.0 1000.0 100.0 100.0 100.0) true)
  (`SkeletalMeshComponent.SetAllBodiesBelowSimulatePhysics` (`self.Mesh`) _pelvisbone true false))

(event `EnhancedInput|/Game/CharacterPlayer/Input/IA_Grab`
  (params (ActionValue :type Boolean) (ElapsedSeconds :type "Float (double-precision)") (TriggeredSeconds :type "Float (double-precision)") (InputAction :type "InputAction Object Reference" :default "/Game/CharacterPlayer/Input/IA_Grab.IA_Grab"))
  (bind _returnvalue (`self.K2_GetActorLocation`))
  (:`Triggered`
    (bind (_outhit _returnvalue_2) (`KismetSystemLibrary.SphereTraceSingleForObjects` :`Start` _returnvalue :`End` _returnvalue :`Radius` 100.0 :`ObjectTypes` (`|MakeArray` "ObjectTypeQuery4" :!type "EObjectTypeQuery Enum") :`DrawDebugType` "ForDuration"))
    (if _returnvalue_2
      (`PhysicsConstraintComponent.SetConstrainedComponents` (`self.PhysicsConstraint`) (`self.Mesh`) "spine_05" (`.HitComponent` (`GameplayStatics.BreakHitResult` _outhit)) "None")
      (set `self.isGrabbing` true)
      (else
        (set `self.isGrabbing` false))))
  (:`Completed`
    (set `self.isGrabbing` false)
    (`PhysicsConstraintComponent.BreakConstraint` (`self.PhysicsConstraint`))))

(fn `UserConstructionScript`)